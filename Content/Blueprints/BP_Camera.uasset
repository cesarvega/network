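; BP_Camera is a shared camera for up to four players, set as every PlayerController's view target.
; After a short BeginPlay delay, it caches players from BP_GameMode and starts a looping UpdateCamera timer.
; Helper functions interpolate toward the players' average position and size the spring arm by clamped maximum pairwise distance.
; However, UpdateCamera is empty and both helper calls are disconnected, so neither tracking nor zoom runs.
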(event Custom|UpdateCamera)

(event EventBeginPlay
  (Utilities|FlowControl|Delay 0.01)
  (CallFunction|ClassSetup)
  (Utilities|Time|SetTimerbyFunctionName 0 "UpdateCamera" 0.01 true))

(fn ConstructionScript)

(fn ClassSetup
  (bind _asbp_game_mode (Utilities|Casting|CastToBP_GameMode (Game|GetGameMode)))
  (bind _output_get (Variables|Default|SetBP_GameMode _asbp_game_mode))
  (Variables|Default|SetplayersReference (Variables|/Game/Blueprints/BP_GameMode.BP_GameMode_C|Getplayers _output_get))
  (bind _outactors (Actor|GetAllActorsOfClass "/Script/Engine.PlayerController"))
  (Game|Player|SetViewTargetwithBlend _outactors self 0.0 "VTBlend_Linear" 0.0 false)
  (for (_array_element _array_index) (Variables|Default|GetplayersReference)
    (switch int _array_index
      (:0
        (Variables|Default|Setp1 _array_element))
      (:1
        (Variables|Default|Setp2 _array_element))
      (:2
        (Variables|Default|Setp3 _array_element))
      (:3
        (Variables|Default|Setp4 _array_element)))))

(fn SetArmLength
  (bind _p1 (Variables|Default|Getp1))
  (bind _p2 (Variables|Default|Getp2))
  (bind _p3 (Variables|Default|Getp3))
  (bind _p4 (Variables|Default|Getp4))
  (Variables|/Script/Engine.SpringArmComponent|SetTargetArmLength (Variables|Default|GetSpringArm) (Math|Float|Clamp(Float) (.MaxValue (Math|Float|MaxOfFloatArray (Utilities|Array|MakeArray (CallFunction|CalculateDistance _p1 _p2) (CallFunction|CalculateDistance _p2 _p3) (CallFunction|CalculateDistance _p2 _p4) (CallFunction|CalculateDistance _p3 _p4) (CallFunction|CalculateDistance _p1 _p3) (CallFunction|CalculateDistance _p1 _p4)))) (Variables|Default|GetMinArmLength) (Variables|Default|GetMaxArmLength))))

(fn SetCameraPos
  (Variables|Default|SetCurrentPos (/ (+ (CallFunction|GetLocation (Variables|Default|Getp1)) (CallFunction|GetLocation (Variables|Default|Getp2)) (CallFunction|GetLocation (Variables|Default|Getp3)) (CallFunction|GetLocation (Variables|Default|Getp4))) (Math|Conversions|ToFloat(Integer) (Utilities|Array|Length (Variables|Default|GetplayersReference)))))
  (Transformation|SetActorLocation (Math|Interpolation|VInterpTo (Variables|Default|GetPreviousPos) (Variables|Default|GetCurrentPos) (Utilities|Time|GetWorldDeltaSeconds) (Variables|Default|GetEnterSpeed)) false false)
  (Variables|Default|SetPreviousPos (Transformation|GetActorLocation)))

(fn GetLocation
  (params (Player :type BP%20Player%20Object%20Reference))
  (Utilities|IsValid Player
    (:Is%20Valid
      (LocalVariables|Setlocation (Transformation|GetActorLocation Player)))
    (:Is%20Not%20Valid
      (LocalVariables|Setlocation "0, 0, 0")))
  (return (LocalVariables|Getlocation)))

(fn CalculateDistance
  (params (playerRef1 :type BP%20Player%20Object%20Reference) (playerRef2 :type BP%20Player%20Object%20Reference))
  (if (and (Utilities|IsValid playerRef1) (Utilities|IsValid playerRef2))
    (LocalVariables|SetDistance (Transformation|GetDistanceTo playerRef1 playerRef2))
    (else
      (LocalVariables|SetDistance 0.0)))
  (return (LocalVariables|GetDistance)))